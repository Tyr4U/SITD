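; BP_DOORTEST is a test interactable that swings a pivot component through a quarter turn, apparently as a falling-wood or door motion.
; On BeginPlay it caches the pivot's relative rotation and derives an end rotation offset in pitch.
; Interact plays the TL_Fallingwood timeline from the start, lerping the pivot between the two rotations.
; It has no reverse or toggle, so each interaction replays the same motion.
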(event EventBeginPlay
  (|CallParentFunction)
  (bind _output_get (Variables|Default|SetStartingRotation (Variables|/Script/Engine.SceneComponent|GetRelativeRotation (Variables|Default|GetPivot))))
  (Variables|Default|SetEndingRot (Math|Rotator|MakeRotator (.Roll (Math|Rotator|BreakRotator _output_get)) (+ (.Pitch (Math|Rotator|BreakRotator _output_get)) -9e+01) (.Yaw (Math|Rotator|BreakRotator _output_get)))))

(event Collision|EventActorBeginOverlap
  (params (OtherActor :type Actor%20Object%20Reference))
  (|CallParentFunction OtherActor) ; This node is disabled and will not be called.\nDrag off pins to build functionality.
)

(event EventTick
  (params (DeltaSeconds :type Float%20%28single-precision%29))
  (|CallParentFunction DeltaSeconds) ; This node is disabled and will not be called.\nDrag off pins to build functionality.
)

(event EventInteract
  (bind _alpha (Timeline|TL_Fallingwood PlayFromStart)
    (:Update
      (Transformation|SetRelativeRotation (Variables|Default|GetPivot) (Math|Rotator|Lerp(Rotator) (Variables|Default|GetStartingRotation) (Variables|Default|GetEndingRot) _alpha) false false))))

(fn ConstructionScript
  (|CallParentFunction))