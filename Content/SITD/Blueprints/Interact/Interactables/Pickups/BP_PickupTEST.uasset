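; Test pickup interactable that the player can take into the first-person right hand.
; Interact turns off physics and collision on Object, snaps the pickup to the hand_R socket of the player's first-person mesh, and registers it as the held item.
; Use is an empty event.
; Drop logic that detaches, restores physics and collision, and clears the held item exists but is unconnected, so it never runs.
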(event EventBeginPlay
  (|CallParentFunction) ; This node is disabled and will not be called.\nDrag off pins to build functionality.
)

(event Collision|EventActorBeginOverlap
  (params (OtherActor :type Actor%20Object%20Reference))
  (|CallParentFunction OtherActor) ; This node is disabled and will not be called.\nDrag off pins to build functionality.
)

(event EventTick
  (params (DeltaSeconds :type Float%20%28single-precision%29))
  (|CallParentFunction DeltaSeconds) ; This node is disabled and will not be called.\nDrag off pins to build functionality.
)

(event EventInteract
  (bind _player_ref (Variables|Default|GetPlayer%20Ref))
  (bind _object (Variables|Default|GetObject))
  (Physics|SetSimulatePhysics _object false)
  (Collision|SetCollisionEnabled (Variables|Default|GetObject) "NoCollision")
  (if (not (Physics|IsSimulatingPhysics _object "None"))
    (Transformation|AttachComponentToComponent (Variables|/Game/SITD/Blueprints/PC/BP_V1ct1m.BP_V1ct1m_C|GetFirstPersonMesh _player_ref) "hand_R" "SnapToTarget" "SnapToTarget" "KeepWorld" true)
    (Transformation|SetRelativeLocation (Variables|Default|GetObject) "0, 0, 0" false false)
    (Default|SetHeldItem _player_ref self)))

(event EventUse)

(fn ConstructionScript
  (|CallParentFunction))