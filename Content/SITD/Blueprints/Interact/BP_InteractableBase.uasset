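; BP_InteractableBase is the base Blueprint for objects the player can look at and interact with in SITD.
; On BeginPlay it caches GI_SITD and its player reference, and binds to OnPlayerReady to refresh that reference when the player becomes ready.
; Look passes the object's InteractType to the player's HUD through ChangeLookAt.
; Interact is an empty event, leaving the base with no interaction behavior of its own.
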(event Custom|PlayerRef
  (Variables|Default|SetPlayer%20Ref (Variables|/Game/SITD/Blueprints/Core/GI_SITD.GI_SITD_C|GetPlayer%20Ref (Variables|Default|GetGameInstance))))

(event EventBeginPlay
  (bind _asgi_sitd (Utilities|Casting|CastToGI_SITD (Game|GetGameInstance)))
  (Variables|Default|SetGameInstance _asgi_sitd)
  (Utilities|IsValid (Variables|/Game/SITD/Blueprints/Core/GI_SITD.GI_SITD_C|GetPlayer%20Ref _asgi_sitd)
    (:Is%20Valid
      (Variables|Default|SetPlayer%20Ref (Variables|/Game/SITD/Blueprints/Core/GI_SITD.GI_SITD_C|GetPlayer%20Ref _asgi_sitd)))
    (:Is%20Not%20Valid
      _))
  (EventDispatchers|BindEventtoOnPlayerReady (Variables|Default|GetGameInstance) (delegate Custom|PlayerRef)))

(event Collision|EventActorBeginOverlap
  (params (OtherActor :type Actor%20Object%20Reference)))

(event EventTick
  (params (DeltaSeconds :type Float%20%28single-precision%29)))

(event EventLook
  (Default|ChangeLookat (Variables|/Game/SITD/Blueprints/PC/BP_V1ct1m.BP_V1ct1m_C|GetHud (Variables|Default|GetPlayer%20Ref)) (Variables|Default|GetInteract%20Type)))

(event EventInteract)

(fn ConstructionScript)