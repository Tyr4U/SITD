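; First-person player character for SITD: collects evidence to win at three pieces, and dies when fear runs out.
; A per-tick camera trace finds interactables, mouse-wheel slots load and spawn held items from soft class references, and timers drain or restore fear.
; Death records a floor-traced location in the game instance, respawned as markers on BeginPlay, then shows the restart widget.
; Also handles stamina-based sprinting, pause and a flashlight montage toggle.
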(event Custom|PlayerStamina
  ;[0.1169 1 0 0.5] Stamina
  (Variables|CharacterStats|SetStamina (Variables|CharacterStats|GetMaxStamina)))

(event Custom|SanityLimit
  ;[0.1169 1 0 0.5] Sanity Limit
  (Variables|CharacterStats|SetFear (Variables|CharacterStats|GetMaxFear)))

(event Custom|CountEvidence
  ;[0.1169 1 0 0.5] Collection System for Evidence
  (bind _result (Math|Integer|IncrementInt (Variables|Default|GetEvidenceCollected))
    (:%20%20
      (if (>= _result 3)
        (Utilities|FlowControl|Sequence
          (:then_0
            (bind _returnvalue (UserInterface|CreateWidget "/Game/SITD/Blueprints/Widgets/HUD/WBP_Win.WBP_Win_C"))
            (UserInterface|Viewport|AddtoViewport _returnvalue 0)
            (CallFunction|HandleWin)))
        (else
          ;;[0 0 0 0.5] Iterations for evidence collection
          (if (>= (Variables|Default|GetEvidenceCollected) 1)
            (bind _returnvalue_2 (UserInterface|CreateWidget "/Game/SITD/Blueprints/Widgets/HUD/WBP_ObjectiveWidget.WBP_ObjectiveWidget_C"))
            (UserInterface|Viewport|AddtoViewport _returnvalue_2 0)
            (Utilities|FlowControl|Delay 5.0)
            (Widget|RemovefromParent _returnvalue_2)))))))

(event Custom|NoFearTimer
  ;[0 0.8715 1 0.5] Fear System
  ;;[0.1169 1 0 0.5] Raise the Fear Bar
  (Variables|CharacterStats|SetFear (Math|Float|Clamp(Float) (+ (Variables|CharacterStats|GetFear) 0.01))))

(event Custom|ScaredTimer
  ;[0 0.8715 1 0.5] Fear System
  ;;[0.1169 1 0 0.5] Drain Fear Bar
  (bind _output_get (Variables|CharacterStats|SetFear (Math|Float|Clamp(Float) (- (Variables|CharacterStats|GetFear) 0.001))))
  (if (<= _output_get 0.0)
    (Utilities|FlowControl|DoOnce false
      (:Completed
        (CallFunction|Death)))))

(event Custom|SetHeldItem
  (params (Held%20Item :type BP%20Interactable%20Base%20Object%20Reference))
  (bind _returnvalue (Utilities|GetClass Held%20Item))
  (bind _output (Utilities|ResolveSoftReference _returnvalue))
  (Variables|Default|SetMatchFound false)
  (bind _array_element (Utilities|Array|ForEachLoopwithBreak (Variables|Default|GetInventory) :!label _label)
    (:LoopBody
      (if (== _array_element _output)
        (Variables|Default|SetMatchFound true)
        (goto _label Break)))
    (:Completed
      (if (Variables|Default|GetMatchFound)
        (Variables|Default|SetHeldItem Held%20Item)
        (else
          (bind (_array_element_2 _array_index) (Utilities|Array|ForEachLoopwithBreak (Variables|Default|GetInventory) :!label _label_2)
            (:LoopBody
              (if (not (Utilities|IsValidSoftClassReference _array_element_2))
                (if (== _array_index (Variables|Default|GetSelectedSlots))
                  (Variables|Default|SetHeldItem Held%20Item))
                (Utilities|Array|SetArrayElem (Variables|Default|GetInventory) _array_index _output)
                (Default|SetInventory (Variables|Default|GetHud) _array_index)
                (goto _label_2 Break)))))))))

(event Custom|RefillStamina
  ;[0.1169 1 0 0.5] Sprint IF Stamina is > than 0, IF stamina is <= to 0 then refill stamina
  ;;[0 0 0 0.5] Refill
  (Variables|CharacterStats|SetStamina (+ (Variables|CharacterStats|GetStamina) 0.01)))

(event Custom|PlayerDeath
  (bind _returnvalue (Transformation|GetActorLocation))
  (bind _returnvalue_2 (Transformation|GetActorRotation))
  (bind _as_gi_sitd (Variables|Default|GetAs%20GI%20SITD))
  (Math|Integer|IncrementInt (Variables|Default|GetDeaths)
    (:%20%20
      ;[0.15 0.15 0.15 0.5] Places a Death marker on the ground where player has died.
      (bind _outhit (Collision|LineTraceByChannel _returnvalue (+ (* (Math|Vector|NegateVector (Transformation|GetActorUpVector)) 5e+02) _returnvalue) "TraceTypeQuery1" false 0 "ForDuration"))
      (Default|AddDeathLocation _as_gi_sitd (Utilities|Struct|MakeS_Deaths (.Location (Collision|BreakHitResult _outhit)) _returnvalue_2 (+ (Utilities|Array|Length (Variables|/Game/SITD/Blueprints/Core/GI_SITD.GI_SITD_C|GetDeaths _as_gi_sitd)) 1)))
      (bind _returnvalue_3 (Game|SpawnActorfromClass "/Game/SITD/Blueprints/Core/Death/BP_DeathMarker.BP_DeathMarker_C" (Math|Transform|MakeTransform (.Location (Collision|BreakHitResult _outhit)) _returnvalue_2 "1.000000,1.000000,1.000000") "Undefined" "MultiplyWithRoot" 0 0))
      (Default|SetMarkerText _returnvalue_3 (Utilities|String|ToString(Integer) (Variables|Default|GetDeaths))))))

(event Custom|ClearSlot
  (bind _selectedslots (Variables|Default|GetSelectedSlots))
  (Utilities|Array|RemoveIndex (Variables|Default|GetInventory) _selectedslots)
  (Default|ClearInventorySlot (Variables|Default|GetHud) _selectedslots)
  (CallFunction|ClearHeldItem))

(event Custom|Clear%20Held%20Item
  (Variables|Default|SetHeldItem 0))

(event Custom|Death
  (bind _returnvalue (Game|GetPlayerController 0))
  ;[0 0.8715 1 0.5] On Death Event
  (CallFunction|PlayerDeath)
  (Components|Activation|Deactivate (Variables|Default|GetFirstPersonCamera))
  (Default|CallOnPlayerDeath self)
  (Components|Activation|Activate (Variables|Default|GetDeathCam) false)
  ;;[0 0 0 0.5] Play Scared Sound
  (Audio|PlaySound2D "/Game/SITD/Sounds/MaleScream.MaleScream" 1.0 1.0 0.0 0 0)
  (Input|DisableInput (Game|GetPlayerController 0))
  (Utilities|FlowControl|DoOnce false
    (:Completed
      (Components|Animation|PlayAnimation (Variables|Character|GetMesh) "/Game/SITD/Animations/Death_Anim_Anim.Death_Anim_Anim" false)
      (Variables|Default|Set?IsDead true)
      (Utilities|FlowControl|Delay 5.0)
      (Utilities|IsValid _returnvalue
        (:Is%20Valid
          (Variables|/Script/Engine.PlayerController|SetbShowMouseCursor _returnvalue true)
          (Input|SetInputModeUIOnly 0 0 "DoNotLock" false)
          (bind _returnvalue_2 (UserInterface|CreateWidget "/Game/SITD/Blueprints/Widgets/HUD/WBP_RestartWidget.WBP_RestartWidget_C"))
          (UserInterface|Viewport|AddtoViewport _returnvalue_2 0))))))

(event Input|EnhancedActionEvents|EnhancedInputActionIA_Sprint
  (params (ActionValue :type Boolean) (ElapsedSeconds :type Float%20%28double-precision%29) (TriggeredSeconds :type Float%20%28double-precision%29) (InputAction :type Input%20Action%20Object%20Reference :default "/Game/FirstPerson/Input/Actions/IA_Sprint.IA_Sprint"))
  ;[0.1169 1 0 0.5] Sprint IF Stamina is > than 0, IF stamina is <= to 0 then refill stamina
  (:Triggered
    (Variables|CharacterStats|SetbIsSprinting true)
    (if (> (Variables|CharacterStats|GetStamina) 0.0)
      (Variables|CharacterStats|SetbNoStamina false)
      (Variables|CharacterStats|SetStamina (Math|Float|Clamp(Float) (- (Variables|CharacterStats|GetStamina) 0.003)))
      (Variables|/Script/Engine.CharacterMovementComponent|SetMaxWalkSpeed (Variables|Character|GetCharacterMovement) 6e+02)
      (else
        (Variables|CharacterStats|SetbIsSprinting false)
        (Variables|CharacterStats|SetbNoStamina true)
        (Variables|/Script/Engine.CharacterMovementComponent|SetMaxWalkSpeed (Variables|Character|GetCharacterMovement) 3e+02))))
  (:Canceled
    (Variables|CharacterStats|SetbIsSprinting false)
    (if (< (Variables|CharacterStats|GetStamina) 1.0) :!label _label
      (Variables|/Script/Engine.CharacterMovementComponent|SetMaxWalkSpeed (Variables|Character|GetCharacterMovement) 3e+02 :!label _label_2)
      (Utilities|FlowControl|RetriggerableDelay 0.2)
      (CallFunction|RefillStamina)
      (goto _label_2)))
  (:Completed
    (Variables|CharacterStats|SetbIsSprinting false)
    (goto _label)))

(event Input|EnhancedActionEvents|EnhancedInputActionIA_Pause
  (params (ActionValue :type Boolean) (ElapsedSeconds :type Float%20%28double-precision%29) (TriggeredSeconds :type Float%20%28double-precision%29) (InputAction :type Input%20Action%20Object%20Reference :default "/Game/FirstPerson/Input/Actions/IA_Pause.IA_Pause"))
  (bind _returnvalue (Game|GetPlayerController 0))
  (bind _returnvalue_2 (Game|GetPlayerController 0))
  ;[0.1169 1 0 0.5] Handle Puase
  (:Started
    (Utilities|IsValid (Variables|Default|GetPauseRef)
      (:Is%20Valid
        _)
      (:Is%20Not%20Valid
        (bind _returnvalue_3 (UserInterface|CreateWidget "/Game/SITD/Blueprints/Widgets/HUD/WBP_Pause.WBP_Pause_C"))
        (Variables|Default|SetPauseRef _returnvalue_3)))
    (if (Game|IsGamePaused)
      ;;[0 0.8715 1 0.5] IF game is Paused True on P press Set to False and DO NOT show Mouse Cursor
      (Widget|RemovefromParent (Variables|Default|GetPauseRef))
      (Game|SetGamePaused false)
      (Variables|/Script/Engine.PlayerController|SetbShowMouseCursor _returnvalue false)
      (Input|SetInputModeGameOnly _returnvalue false)
      (else
        (UserInterface|Viewport|AddtoViewport (Variables|Default|GetPauseRef) 0)
        (Game|SetGamePaused true)
        (Variables|/Script/Engine.PlayerController|SetbShowMouseCursor _returnvalue_2 true)
        (Input|SetInputModeGameandUI _returnvalue_2 (Variables|Default|GetPauseRef) "DoNotLock" true false)))))

(event EventBeginPlay
  ;[0.15 0.15 0.15 0.5] Handle Events on Begin play
  (Utilities|FlowControl|Sequence
    (:then_0
      ;;[0.15 0.15 0.15 0.5] Sends Player Ref to Game instance
      (CallFunction|HandleGameInstance)
      ;;[0.15 0.15 0.15 0.5] Player Stamina and Wellness
      (CallFunction|PlayerStamina)
      (CallFunction|SanityLimit)
      (for _array_element (Variables|/Game/SITD/Blueprints/Core/GI_SITD.GI_SITD_C|GetDeaths (Variables|Default|GetAs%20GI%20SITD))
        (bind _returnvalue (Game|SpawnActorfromClass "/Game/SITD/Blueprints/Core/Death/BP_DeathMarker.BP_DeathMarker_C" (Math|Transform|MakeTransform (.postion _array_element) (.rotation _array_element) "1.000000,1.000000,1.000000") "Undefined" "MultiplyWithRoot" 0 0))
        (Default|SetMarkerText _returnvalue)))
    (:then_1
      ;;[0 0 0 0.5] IF IsInMainMenu True display Objective widget for 5 seconds than Remove from Parent
      (if (Variables|/Game/SITD/Blueprints/PC/BP_V1ct1mController.BP_V1ct1mController_C|GetbIsInMainMenu (.AsBP%20V1ct%201m%20Controller (Utilities|Casting|CastToBP_V1ct1mController (Game|GetPlayerController 0))))
        (bind _returnvalue_2 (UserInterface|CreateWidget "/Game/SITD/Blueprints/Widgets/HUD/WBP_ObjectiveWidget.WBP_ObjectiveWidget_C"))
        (bind _output_get (Variables|Default|SetVHSHUD _returnvalue_2))
        (UserInterface|Viewport|AddtoViewport _output_get 0)
        (Utilities|FlowControl|Delay 5.0)
        (bind _vhshud (Variables|Default|GetVHSHUD)
          (:then
            (Widget|RemovefromParent _vhshud))
          (:else))))))

(event EventTick
  (params (DeltaSeconds :type Float%20%28single-precision%29))
  (bind (_start _end) (CallFunction|StartEndOfLineTraceforInteraction))
  ;[0.15 0.01236 0.1283 0.5] RayTrace For Interaction
  (bind _outhit (Collision|LineTraceByChannel _start _end "TraceTypeQuery1" true 0 "None"))
  (bind _asbp_interactable_base (Utilities|Casting|CastToBP_InteractableBase (.HitActor (Collision|BreakHitResult _outhit)))
    (:then
      (Default|Look _asbp_interactable_base)
      (Variables|Default|SetCanInteract true)
      (Variables|Default|SetLookedAtThing _asbp_interactable_base))
    (:CastFailed
      (bind _hud (Variables|Default|GetHud)
        (:then
          (Default|ChangeLookat _hud "NewEnumerator5")
          (Variables|Default|SetCanInteract false))
        (:else)))))

(event EventNoFear
  ;[0 0.8715 1 0.5] Fear System
  ;;[0.1169 1 0 0.5] Raise the Fear Bar
  (if (not (Variables|Default|GetbFeared))
    (bind _returnvalue (Utilities|Time|SetTimerbyEvent (delegate Custom|NoFearTimer) 0.1 true))
    (Variables|Default|SetFearTime _returnvalue)))

(event EventScared
  ;[0 0.8715 1 0.5] Fear System
  ;;[0.1169 1 0 0.5] Drain Fear Bar
  (if (and (> (Variables|CharacterStats|GetFear) 0.0) (Variables|Default|GetbFeared))
    (bind _returnvalue (Utilities|Time|SetTimerbyEvent (delegate Custom|ScaredTimer) 0.2 true))
    (Variables|Default|SetScaredTime _returnvalue)
    (else
      (CallFunction|PlayerDeath))))

(event Input|KeyboardEvents|G
  (params (Key :type Key%20Structure :default "None"))
  (:Pressed
    (CallFunction|Death)))

(event Input|MouseEvents|MouseWheelUp
  (params (Key :type Key%20Structure :default "None"))
  (bind _selectedslots (Variables|Default|GetSelectedSlots))
  ;[0.1169 1 0 0.5] Slots in Inventory Selected
  (:Pressed
    (if (not (== _selectedslots (Variables|Default|GetMaxSlots)))
      (bind _result (Math|Integer|IncrementInt _selectedslots)
        (:%20%20
          (Default|ChangeSlot (Variables|Default|GetHud) _result)
          (Utilities|IsValid (Variables|Default|GetHeldItem)
            (:Is%20Valid
              (Actor|DestroyActor (Variables|Default|GetHeldItem))
              (CallFunction|ClearHeldItem))
            (:Is%20Not%20Valid
              _))
          (bind _returnvalue (Utilities|LoadClassAssetBlocking (Utilities|Array|Get(acopy) (Variables|Default|GetInventory) (Variables|Default|GetSelectedSlots))))
          (bind _asactor (Utilities|Casting|CastToActorClass _returnvalue))
          (bind _returnvalue_2 (Game|SpawnActorfromClass _asactor (Math|Transform|MakeTransform "0, 0, 0" "0, 0, 0" "1.000000,1.000000,1.000000") "Undefined" "MultiplyWithRoot" 0 0))
          (bind _asbp_interactable_base (Utilities|Casting|CastToBP_InteractableBase _returnvalue_2))
          (Class|BPIInteract|Interact(Message) _asbp_interactable_base)
          (Collision|SetActorEnableCollision _asbp_interactable_base true)
          (Variables|Default|SetHeldItem _asbp_interactable_base))))))

(event Input|MouseEvents|MouseWheelDown
  (params (Key :type Key%20Structure :default "None"))
  (bind _selectedslots (Variables|Default|GetSelectedSlots))
  ;[0.1169 1 0 0.5] Slots in Inventory Selected
  (:Pressed
    (if (not (== _selectedslots 0))
      (bind _result (Math|Integer|DecrementInt _selectedslots)
        (:%20%20
          (Default|ChangeSlot (Variables|Default|GetHud) _result)
          (Utilities|IsValid (Variables|Default|GetHeldItem)
            (:Is%20Valid
              (Actor|DestroyActor (Variables|Default|GetHeldItem))
              (CallFunction|ClearHeldItem))
            (:Is%20Not%20Valid
              _))
          (bind _returnvalue (Utilities|LoadClassAssetBlocking (Utilities|Array|Get(acopy) (Variables|Default|GetInventory) (Variables|Default|GetSelectedSlots))))
          (bind _asactor (Utilities|Casting|CastToActorClass _returnvalue))
          (bind _returnvalue_2 (Game|SpawnActorfromClass _asactor (Math|Transform|MakeTransform "0, 0, 0" "0, 0, 0" "1.000000,1.000000,1.000000") "Undefined" "MultiplyWithRoot" 0 0))
          (bind _asbp_interactable_base (Utilities|Casting|CastToBP_InteractableBase _returnvalue_2))
          (Class|BPIInteract|Interact(Message) _asbp_interactable_base)
          (Collision|SetActorEnableCollision _asbp_interactable_base true)
          (Variables|Default|SetHeldItem _asbp_interactable_base))))))

(event Input|KeyboardEvents|R
  (params (Key :type Key%20Structure :default "None"))
  ;[0.15 0 0 0.5] Flashlight Idle
  (:Pressed
    (Utilities|FlowControl|FlipFlop
      (:A
        (Animation|Montage|PlayMontage (Variables|Character|GetMesh) "/Game/SITD/Animations/Flashlight_Idle_Montage.Flashlight_Idle_Montage"))
      (:B
        (Animation|Montage|MontageStop (Components|SkeletalMesh|GetAnimInstance (Variables|Character|GetMesh)) 0.0 "/Game/SITD/Animations/Flashlight_Idle_Montage.Flashlight_Idle_Montage")))))

(fn ConstructionScript)

(fn HandleWidgets)

(fn HandleGameInstance
  (bind _asgi_sitd (Utilities|Casting|CastToGI_SITD (Game|GetGameInstance)))
  (Variables|Default|SetAs%20GI%20SITD _asgi_sitd)
  (Default|SetPlayerRef _asgi_sitd self)
  (bind _asgm_sitd (Utilities|Casting|CastToGM_SITD (Game|GetGameMode)))
  (Variables|/Game/SITD/Blueprints/GameMode/GM_SITD.GM_SITD_C|SetRespawnPoint _asgm_sitd (Transformation|GetActorTransform)))

(fn StartEndOfLineTraceforInteraction
  (bind _returnvalue (Transformation|GetActorLocation))
  (bind _baseeyeheight (Variables|Default|GetBaseEyeHeight))
  (bind _returnvalue_2 (Math|Vector|MakeVector 0.0 0.0 _baseeyeheight))
  (bind _returnvalue_3 (+ _returnvalue _returnvalue_2))
  (return _returnvalue_3 (+ _returnvalue_3 (* (Transformation|GetActorForwardVector (Game|GetPlayerCameraManager 0)) 1e+03))))

(fn HandleWin
  (bind _returnvalue (Game|GetPlayerController 0))
  (bind _returnvalue_2 (UserInterface|CreateWidget "/Game/SITD/Blueprints/Widgets/HUD/WBP_Win.WBP_Win_C"))
  (bind _output_get (Variables|Default|SetWinHud _returnvalue_2))
  (UserInterface|Viewport|AddtoViewport _output_get 0)
  (Variables|/Script/Engine.PlayerController|SetbShowMouseCursor _returnvalue true)
  (Input|SetInputModeGameandUI _returnvalue _returnvalue_2 "DoNotLock" true false))

(fn HandleWidgets)