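; Player controller for the SITD player character, translating Enhanced Input into looking, movement, interaction and held-item drop and use.
; On BeginPlay it shows the HUD widget if in the main menu, gets the player from GI_SITD, adds the input mapping and caches the pawn.
; Movement follows control rotation, while interact, drop and attack message the player's looked-at or held object.
; ToggleHud switches between game-only and UI-only input, creating a new HUD widget each time.
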(event Custom|PlayerRef
  ;[0 0.6875 0.04653 0.5] Event Bein Events
  (Variables|Default|SetPlayer%20Ref (Variables|/Game/SITD/Blueprints/Core/GI_SITD.GI_SITD_C|GetPlayer%20Ref (Variables|Default|GetGameInstance))))

(event Custom|ToggleHud
  ;[0 0.8715 1 0.5] Toggle Hud On/Off depending on if in Menu or not
  (if (Variables|Default|GetbIsInMainMenu)
    (bind _returnvalue (UserInterface|CreateWidget "/Game/SITD/Blueprints/Widgets/HUD/WBP_HUD1.WBP_HUD1_C"))
    (Utilities|IsValid _returnvalue
      (:Is%20Valid
        (UserInterface|Viewport|AddtoViewport _returnvalue 0)
        (Variables|Default|SetbIsInMainMenu false)
        (Widget|SetVisibility _returnvalue "Hidden")
        (Input|SetInputModeGameOnly self false)))
    (else
      (bind _returnvalue_2 (UserInterface|CreateWidget "/Game/SITD/Blueprints/Widgets/HUD/WBP_HUD1.WBP_HUD1_C"))
      (Utilities|IsValid _returnvalue_2
        (:Is%20Valid
          (UserInterface|Viewport|AddtoViewport _returnvalue_2 0)
          (Variables|Default|SetbIsInMainMenu true)
          (Widget|SetVisibility _returnvalue_2 "Visible")
          (Variables|/Script/Engine.PlayerController|SetbShowMouseCursor (Game|GetPlayerController 0) true)
          (Input|SetInputModeUIOnly self (Variables|Default|GetHUD) "DoNotLock" false))))))

(event Input|EnhancedActionEvents|EnhancedInputActionIA_Move
  (params (ActionValue :type Vector%202D%20Structure) (ElapsedSeconds :type Float%20%28double-precision%29) (TriggeredSeconds :type Float%20%28double-precision%29) (InputAction :type Input%20Action%20Object%20Reference :default "/Game/FirstPerson/Input/Actions/IA_Move.IA_Move"))
  ;[0 0.6875 0.04653 0.5] Handle Movement
  (Movement|HandleMovement))

(event Input|EnhancedActionEvents|EnhancedInputActionIA_Interact
  (params (ActionValue :type Boolean) (ElapsedSeconds :type Float%20%28double-precision%29) (TriggeredSeconds :type Float%20%28double-precision%29) (InputAction :type Input%20Action%20Object%20Reference :default "/Game/FirstPerson/Input/Actions/IA_Interact.IA_Interact"))
  (bind _player_ref (Variables|Default|GetPlayer%20Ref))
  (:Started
    (if (Variables|/Game/SITD/Blueprints/PC/BP_V1ct1m.BP_V1ct1m_C|GetCanInteract _player_ref)
      (bind _lookedatthing (Variables|/Game/SITD/Blueprints/PC/BP_V1ct1m.BP_V1ct1m_C|GetLookedAtThing _player_ref)
        (:then
          (Class|BPIInteract|Interact(Message) _lookedatthing))
        (:else)))))

(event Input|EnhancedActionEvents|EnhancedInputActionIA_Drop
  (params (ActionValue :type Boolean) (ElapsedSeconds :type Float%20%28double-precision%29) (TriggeredSeconds :type Float%20%28double-precision%29) (InputAction :type Input%20Action%20Object%20Reference :default "/Game/FirstPerson/Input/Actions/IA_Drop.IA_Drop"))
  (bind _player_ref (Variables|Default|GetPlayer%20Ref))
  (bind _helditem (Variables|/Game/SITD/Blueprints/PC/BP_V1ct1m.BP_V1ct1m_C|GetHeldItem _player_ref))
  (:Started
    (Utilities|IsValid _helditem
      (:Is%20Valid
        (Default|DropItem _helditem)))))

(event Input|EnhancedActionEvents|EnhancedInputActionIA_Attack
  (params (ActionValue :type Boolean) (ElapsedSeconds :type Float%20%28double-precision%29) (TriggeredSeconds :type Float%20%28double-precision%29) (InputAction :type Input%20Action%20Object%20Reference :default "/Game/FirstPerson/Input/Actions/IA_Attack.IA_Attack"))
  (bind _player_ref (Variables|Default|GetPlayer%20Ref))
  (bind _helditem (Variables|/Game/SITD/Blueprints/PC/BP_V1ct1m.BP_V1ct1m_C|GetHeldItem _player_ref))
  (Utilities|IsValid _helditem
    (:Is%20Valid
      (Class|BPIInteract|Use(Message) _helditem))))

(event Input|EnhancedActionEvents|EnhancedInputActionIA_MouseLook
  (params (ActionValue :type Vector%202D%20Structure) (ElapsedSeconds :type Float%20%28double-precision%29) (TriggeredSeconds :type Float%20%28double-precision%29) (InputAction :type Input%20Action%20Object%20Reference :default "/Game/FirstPerson/Input/Actions/IA_MouseLook.IA_MouseLook"))
  ;[0 0.6875 0.04653 0.5] Handle Look
  (Movement|MouseHandleLook ActionValue))

(event Input|EnhancedActionEvents|EnhancedInputActionIA_AnalogLook
  (params (ActionValue :type Vector%202D%20Structure) (ElapsedSeconds :type Float%20%28double-precision%29) (TriggeredSeconds :type Float%20%28double-precision%29) (InputAction :type Input%20Action%20Object%20Reference :default "/Game/FirstPerson/Input/Actions/IA_AnalogLook.IA_AnalogLook"))
  ;[0 0.6875 0.04653 0.5] Handle Look
  (Movement|AnalogHandleLook ActionValue))

(event EventBeginPlay
  ;[0 0.6875 0.04653 0.5] Event Bein Events
  (CallFunction|HandleWidget)
  (bind _asgi_sitd (Utilities|Casting|CastToGI_SITD (Game|GetGameInstance)))
  (Variables|Default|SetGameInstance _asgi_sitd)
  (Utilities|IsValid (Variables|/Game/SITD/Blueprints/Core/GI_SITD.GI_SITD_C|GetPlayer%20Ref _asgi_sitd)
    (:Is%20Valid
      (Variables|Default|SetPlayer%20Ref (Variables|/Game/SITD/Blueprints/Core/GI_SITD.GI_SITD_C|GetPlayer%20Ref _asgi_sitd)))
    (:Is%20Not%20Valid
      _))
  (EventDispatchers|BindEventtoOnPlayerReady (Variables|Default|GetGameInstance) (delegate Custom|PlayerRef))
  (StoredEssentials|HandleMapping)
  (StoredEssentials|StoreMovementComponent))

(fn ConstructionScript)

(fn HandleMapping
  (Input|AddMappingContext (PlayerController|LocalPlayerSubsystems|GetEnhancedInputLocalPlayerSubsystem) "/Game/FirstPerson/Input/IMC_Default.IMC_Default" 0 "(bIgnoreAllPressedKeysUntilRelease=True,bForceImmediately=False,bNotifyUserSettings=False)"))

(fn StoreMovementComponent
  (bind _ascharacter (Utilities|Casting|CastToCharacter (Game|Player|GetPlayerPawn 0)))
  (Variables|StoredEssentials|SetControlledCharacter _ascharacter)
  (Variables|StoredEssentials|SetCharacterMovementComponent (Pawn|GetMovementComponent (Pawn|GetControlledPawn))))

(fn MouseHandleLook
  (params (ActionValues :type Vector%202D%20Structure))
  (bind (_x _y) (Math|Vector2D|BreakVector2D ActionValues))
  ;[0.1169 1 0 0.5] Look with low sensitivity @ .1 float
  (Class|PlayerController|AddYawInput (* _x (Variables|Default|GetVerticalLookSensitivity)))
  (Class|PlayerController|AddPitchInput (* _y (Variables|Default|GetHorizontalLookSensitivity))))

(fn MoveForwardDirection
  ;[0.1169 1 0 0.5] Get and store controlled pawn and its movement component along with the Vector at which the pawn moves
  (return (Pawn|GetMovementComponent (Pawn|GetControlledPawn)) (* (Math|Vector|GetForwardVector (Pawn|GetControlRotation :!class /Script/Engine.Controller)) (.y (Input|EnhancedActionValues|GetIA_Move)))))

(fn MoveRightDirection
  (return (Pawn|GetMovementComponent (Pawn|GetControlledPawn)) (* (Math|Vector|GetRightVector (Pawn|GetControlRotation :!class /Script/Engine.Controller)) (.x (Input|EnhancedActionValues|GetIA_Move)))))

(fn HandleMovement
  (bind (_movementcomponent _xaxis) (Movement|MoveRightDirection))
  (bind (_movementcomponent_2 _yaxis) (Movement|MoveForwardDirection))
  ;[0.1169 1 0 0.5] Validate Controlled Character the Add input vector Forward and Right Direction
  (Variables|StoredEssentials|GetControlledCharacter
    (:then
      (Class|PawnMovementComponent|AddInputVector _movementcomponent_2 _yaxis false)
      (Class|PawnMovementComponent|AddInputVector _movementcomponent _xaxis false))
    (:else)))

(fn HandleWidget
  (if (Variables|Default|GetbIsInMainMenu)
    (bind _returnvalue (UserInterface|CreateWidget "/Game/SITD/Blueprints/Widgets/HUD/WBP_HUD1.WBP_HUD1_C"))
    (UserInterface|Viewport|AddtoViewport _returnvalue 0)))

(fn AnalogHandleLook
  (params (ActionValues :type Vector%202D%20Structure))
  (bind (_x _y) (Math|Vector2D|BreakVector2D ActionValues))
  ;[0.1169 1 0 0.5] Look with low sensitivity @ .3 float
  (Class|PlayerController|AddYawInput (* _x (Variables|Default|GetVerticalLookSensitivity)))
  (Class|PlayerController|AddPitchInput (* _y (Variables|Default|GetHorizontalLookSensitivity))))