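; BP_GameStarter randomly places the game's evidence and pickup items on BeginPlay.
; It pairs each Evidence and Pickups entry with a random BP_ItemPlacer, then SetItems spawns them at those transforms.
; Evidence removes its used placer from the pool, while Pickups removes a freshly randomized one.
; PlayerRest destroys spawned items and reruns placement without clearing prior pairings; its player-death binding is unconnected.
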(event Custom|SetItems
  (for _array_element (Variables|Default|GetSpawnedLocations)
    (bind _returnvalue (Game|SpawnActorfromClass (Utilities|ResolveSoftReference (.spawneditem _array_element)) (Math|Transform|MakeTransform (Transformation|GetActorLocation (.itemlocation _array_element)) (Transformation|GetActorRotation (.itemlocation _array_element)) "1.000000,1.000000,1.000000") "Undefined" "MultiplyWithRoot" 0 0))
    (Utilities|Array|AddUnique (Variables|Default|GetSpawnedItems) _returnvalue)))

(event Custom|OnPlayerReady
  (Variables|Default|SetPlayer%20Ref (Variables|/Game/SITD/Blueprints/Core/GI_SITD.GI_SITD_C|GetPlayer%20Ref (Variables|Default|GetGameInstance))))

(event Custom|PlayerRest
  (for _array_element (Variables|Default|GetSpawnedItems)
    (Utilities|IsValid _array_element
      (:Is%20Valid
        (Actor|DestroyActor _array_element))))
  (bind _outactors (Actor|GetAllActorsOfClass "/Game/SITD/Blueprints/BP_ItemPlacer.BP_ItemPlacer_C"))
  (Variables|Default|SetPlacedLocations _outactors)
  (for _array_element_2 (Variables|Default|GetEvidence)
    (bind _output_get (Variables|Default|SetProposedPairing (Utilities|Struct|MakeS_Assigned (.OutItem (Utilities|Array|Random (Variables|Default|GetPlacedLocations))) _array_element_2)))
    (Utilities|Array|AddUnique (Variables|Default|GetSpawnedLocations) _output_get)
    (Utilities|Array|RemoveItem (Variables|Default|GetPlacedLocations) (.ItemLocation (Utilities|Struct|BreakS_Assigned _output_get))))
  (for _array_element_3 (Variables|Default|GetPickups)
    (bind _output_get_2 (Variables|Default|SetProposedPairing (Utilities|Struct|MakeS_Assigned (.OutItem (Utilities|Array|Random (Variables|Default|GetPlacedLocations))) _array_element_3)))
    (Utilities|Array|AddUnique (Variables|Default|GetSpawnedLocations) _output_get_2)
    (Utilities|Array|RemoveItem (Variables|Default|GetPlacedLocations) (.OutItem (Utilities|Array|Random (Variables|Default|GetPlacedLocations)))))
  (CallFunction|SetItems))

(event EventBeginPlay
  (bind _asgi_sitd (Utilities|Casting|CastToGI_SITD (Game|GetGameInstance)))
  (Variables|Default|SetGameInstance _asgi_sitd)
  (Utilities|IsValid (Variables|/Game/SITD/Blueprints/Core/GI_SITD.GI_SITD_C|GetPlayer%20Ref _asgi_sitd)
    (:Is%20Valid
      (Variables|Default|SetPlayer%20Ref (Variables|/Game/SITD/Blueprints/Core/GI_SITD.GI_SITD_C|GetPlayer%20Ref _asgi_sitd)))
    (:Is%20Not%20Valid
      _))
  (EventDispatchers|BindEventtoOnPlayerReady (Variables|Default|GetGameInstance) (delegate Custom|OnPlayerReady))
  (bind _outactors (Actor|GetAllActorsOfClass "/Game/SITD/Blueprints/BP_ItemPlacer.BP_ItemPlacer_C"))
  (Variables|Default|SetPlacedLocations _outactors)
  (for _array_element (Variables|Default|GetEvidence)
    (bind _output_get (Variables|Default|SetProposedPairing (Utilities|Struct|MakeS_Assigned (.OutItem (Utilities|Array|Random (Variables|Default|GetPlacedLocations))) _array_element)))
    (Utilities|Array|AddUnique (Variables|Default|GetSpawnedLocations) _output_get)
    (Utilities|Array|RemoveItem (Variables|Default|GetPlacedLocations) (.ItemLocation (Utilities|Struct|BreakS_Assigned _output_get))))
  (for _array_element_2 (Variables|Default|GetPickups)
    (bind _output_get_2 (Variables|Default|SetProposedPairing (Utilities|Struct|MakeS_Assigned (.OutItem (Utilities|Array|Random (Variables|Default|GetPlacedLocations))) _array_element_2)))
    (Utilities|Array|AddUnique (Variables|Default|GetSpawnedLocations) _output_get_2)
    (Utilities|Array|RemoveItem (Variables|Default|GetPlacedLocations) (.OutItem (Utilities|Array|Random (Variables|Default|GetPlacedLocations)))))
  (CallFunction|SetItems))

(fn ConstructionScript)