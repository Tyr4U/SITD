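; Game mode for SITD that caches the player's BP_V1ct1m character and handles respawning it.
; On BeginPlay it stores the player character as PlayerRef.
; RespawnPlayer spawns a new actor of the passed victim's class at RespawnPoint and has player controller 0 possess it.
; It then clears IsDead on the cached PlayerRef, which is not updated to the new pawn, and restores game-only input.
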(event Custom|RespawnPlayer
  (params (V1ctim :type BP%20V1ct%201m%20Object%20Reference))
  (bind _returnvalue (Game|GetPlayerController 0))
  (bind _respawnpoint (Variables|Default|GetRespawnPoint))
  ;[0.1169 1 0 0.5] Respawn Player at new location
  (bind _returnvalue_2 (Game|SpawnActorfromClass (Utilities|GetClass V1ctim) (Math|Transform|MakeTransform (.location _respawnpoint) (.rotation _respawnpoint) "1.000000,1.000000,1.000000") "Undefined" "MultiplyWithRoot" 0 0))
  (Pawn|Possess _returnvalue _returnvalue_2)
  (bind _playerref (Variables|Default|GetPlayerRef)
    (:then
      (Variables|/Game/SITD/Blueprints/PC/BP_V1ct1m.BP_V1ct1m_C|Set?IsDead _playerref false)
      (Input|SetInputModeGameOnly _returnvalue false))
    (:else)))

(event EventBeginPlay
  ;[0.1169 1 0 0.5] Referances on Begin Play
  (CallFunction|HandleReferances))

(fn ConstructionScript)

(fn HandleReferances
  (bind _asbp_v1ct_1m (Utilities|Casting|CastToBP_V1ct1m (Game|GetPlayerCharacter 0)))
  (Variables|Default|SetPlayerRef _asbp_v1ct_1m))