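; BP_LaughingZone is a trigger zone actor that fills an area with random laughter once the BP_V1ct1m player triggers it.
; An overlap with the LaughingZone component checks that player character zero is BP_V1ct1m, not which actor overlapped, then calls PlaySound.
; PlaySound plays a random laugh at a random point in a box around the actor and re-arms itself on a random timer, with no stop condition.
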(event OnComponentBeginOverlap(LaughingZone)
  (params (OverlappedComponent :type Primitive%20Component%20Object%20Reference) (OtherActor :type Actor%20Object%20Reference) (OtherComp :type Primitive%20Component%20Object%20Reference) (OtherBodyIndex :type Integer) (bFromSweep :type Boolean) (SweepResult :type Hit%20Result%20Structure%20%28by%20ref%29))
  (Utilities|Casting|CastToBP_V1ct1m (Game|GetPlayerCharacter 0))
  (CallFunction|PlaySound))

(event Custom|PlaySound
  (Audio|PlaySoundatLocation (.OutItem (Utilities|Array|Random (Variables|Default|GetVariousLaugh))) (Math|Random|RandomPointinBoundingBox (Transformation|GetActorLocation) (Variables|Default|GetRandomDistance)) "0, 0, 0" 1.0 1.0 0.0 0 0 0 0)
  (Utilities|Time|SetTimerbyEvent (delegate Custom|PlaySound) (Math|Random|RandomFloatinRange (Variables|Default|GetminTimeForSound) (Variables|Default|GetMaxTimeFor%20Sound))))

(event EventBeginPlay)

(fn ConstructionScript)