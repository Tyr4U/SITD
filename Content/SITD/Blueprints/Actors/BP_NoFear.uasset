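; BP_NoFear is a zone actor that toggles the player's fear state as they enter and leave its FearZone.
; BeginPlay caches the player character as BP_V1ct1m.
; Entering clears the player's FearTime timer, sets Feared and calls ScaredMessage.
; Leaving clears the ScaredTime timer, unsets Feared and calls NoFearMessage.
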(event OnComponentBeginOverlap(FearZone)
  (params (OverlappedComponent :type Primitive%20Component%20Object%20Reference) (OtherActor :type Actor%20Object%20Reference) (OtherComp :type Primitive%20Component%20Object%20Reference) (OtherBodyIndex :type Integer) (bFromSweep :type Boolean) (SweepResult :type Hit%20Result%20Structure%20%28by%20ref%29))
  ;[0 0.8715 1 0.5] Overlap Event (FEAR ZONE)
  (if (== OtherActor (Game|GetPlayerCharacter 0))
    (Variables|Default|SetbInZone true)
    (if (Variables|Default|GetbInZone)
      (Utilities|Time|ClearandInvalidateTimerbyHandle (Variables|/Game/SITD/Blueprints/PC/BP_V1ct1m.BP_V1ct1m_C|GetFearTime (Variables|Default|GetPlayerRef)))
      (bind _playerref (Variables|Default|GetPlayerRef)
        (:then
          (Variables|/Game/SITD/Blueprints/PC/BP_V1ct1m.BP_V1ct1m_C|SetbFeared _playerref true)
          (Class|BPIStatus|Scared(Message) _playerref))
        (:else)))))

(event OnComponentEndOverlap(FearZone)
  (params (OverlappedComponent :type Primitive%20Component%20Object%20Reference) (OtherActor :type Actor%20Object%20Reference) (OtherComp :type Primitive%20Component%20Object%20Reference) (OtherBodyIndex :type Integer))
  ;[0 0.8715 1 0.5] Overlap Event (FEAR ZONE)
  (if (== OtherActor (Game|GetPlayerCharacter 0))
    (Variables|Default|SetbInZone false)
    (if (not (Variables|Default|GetbInZone))
      (Utilities|Time|ClearandInvalidateTimerbyHandle (Variables|/Game/SITD/Blueprints/PC/BP_V1ct1m.BP_V1ct1m_C|GetScaredTime (Variables|Default|GetPlayerRef)))
      (Variables|/Game/SITD/Blueprints/PC/BP_V1ct1m.BP_V1ct1m_C|SetbFeared (Variables|Default|GetPlayerRef) false)
      (bind _playerref (Variables|Default|GetPlayerRef)
        (:then
          (Class|BPIStatus|NoFear(Message) _playerref))
        (:else)))))

(event EventBeginPlay
  ;[0.15 0.15 0.15 0.5] Event Begin Events
  (CallFunction|HandleReferances))

(fn ConstructionScript)

(fn HandleReferances
  (bind _asbp_v1ct_1m (Utilities|Casting|CastToBP_V1ct1m (Game|GetPlayerCharacter 0)))
  (Variables|Default|SetPlayerRef _asbp_v1ct_1m))