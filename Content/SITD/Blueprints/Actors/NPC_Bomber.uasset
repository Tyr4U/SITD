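; NPC_Bomber is an enemy pawn that wanders, chases the player on sight and kills them on capsule contact.
; BeginPlay caches the BP_V1ct1m player reference, resets health, triggers a randomly delayed move to a reachable point and binds the hit event.
; The wander move does not re-trigger itself.
; PawnSensing sends AIMoveTo to the player's current location, and a DoOnce-guarded hit calls the player's Death.
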(event OnSeePawn(PawnSensing)
  (params (Pawn :type Pawn%20Object%20Reference))
  ;[0 0.8715 1 0.5] When Enemy Pawn senses by sight the PC the Pawn moves towards teh Player Character
  (Variables|Default|SetbSeePlayer true)
  (AI|AIMoveTo self (Transformation|GetActorLocation (Game|GetPlayerCharacter 0)) 0 5.0 false
    (:OnSuccess
      _)
    (:OnFail
      _))
  (Variables|Default|SetbSeePlayer false))

(event Custom|NPCHealth
  ;[0.1169 1 0 0.5] Health
  (Variables|Default|SetHealth (Variables|Default|GetMaxHealth)))

(event Custom|EnemyMove
  ;[0 0.8715 1 0.5] Enemy AI move to random location at a random time variable
  (Utilities|FlowControl|Delay (Math|Random|RandomFloatinRange 1.2 5.0))
  (Variables|Default|SetbIsMoving true)
  (AI|AIMoveTo self (.RandomLocation (AI|Navigation|GetRandomReachablePointinRadius (Transformation|GetActorLocation) (Variables|Default|GetBomberRadius) 0 0)) 0 5.0 false
    (:OnSuccess
      _)
    (:OnFail
      _))
  (Variables|Default|SetbIsMoving false))

(event Custom|PlayerHit
  (params (HitComponent :type Primitive%20Component%20Object%20Reference) (OtherActor :type Actor%20Object%20Reference) (OtherComp :type Primitive%20Component%20Object%20Reference) (NormalImpulse :type Vector) (Hit :type Hit%20Result%20Structure%20%28by%20ref%29))
  ;[0.15 0.15 0.15 0.5] Event Begint Play
  (if (== OtherActor (Game|GetPlayerCharacter 0))
    (Utilities|FlowControl|DoOnce false
      (:Completed
        (bind _playerref (Variables|Default|GetPlayerRef)
          (:then
            (Default|Death _playerref))
          (:else))))))

(event EventBeginPlay
  ;[0.15 0.15 0.15 0.5] Event Begint Play
  (CallFunction|HandleReferances)
  (CallFunction|EnemyMove)
  (Collision|BindEventtoOnComponentHit (Variables|Collision|GetCapsuleComponent) (delegate Custom|PlayerHit)))

(fn ConstructionScript)

(fn HandleReferances
  (bind _asbp_v1ct_1m (Utilities|Casting|CastToBP_V1ct1m (Game|GetPlayerCharacter 0)))
  (Variables|Default|SetPlayerRef _asbp_v1ct_1m)
  (CallFunction|NPCHealth)
  (CallFunction|EnemyMove))